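; Base weapon Blueprint that fires a round from the skeletal mesh's MuzzleFlash socket when a fire request arrives.
; Each shot spawns a BulletClass actor, plays a fire sound and runs a debug-drawn visibility line trace along the mesh's forward vector.
; The trace, rather than this Blueprint's spawned bullet, drives point damage on hits and reports a damage event for AI perception, crediting the owner's instigator controller.
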(event `OnFireRequested`
  (bind _returnvalue (`SceneComponent.GetSocketTransform` (`self.SkeletalMesh`) "MuzzleFlash" "RTS_World"))
  (`self.FireRound` _returnvalue (`KismetMathLibrary.TransformLocation` _returnvalue)))

(event `FireRound`
  (params (MuzzleTransform :type "Transform Structure (by ref)") (MuzzleLocation :type "Vector Structure (by ref)"))
  (bind _returnvalue (`self.GetInstigatorController` (`self.GetOwner`)))
  (`|SpawnActorFromClass` (`self.Bullet class`) MuzzleTransform "AlwaysSpawn" "OverrideRootScale" null null)
  (`GameplayStatics.PlaySoundAtLocation` "/Game/FPSTemplate/FPWeapon/Audio/FirstPersonTemplateWeaponFire02.FirstPersonTemplateWeaponFire02" MuzzleLocation (struct) 1.0 1.0 0.0 null null null null)
  (bind (_outhit _returnvalue_2) (`KismetSystemLibrary.LineTraceSingle` :`Start` MuzzleLocation :`End` (+ MuzzleLocation (* (`SceneComponent.GetForwardVector` (`self.SkeletalMesh`)) (`self.Range`))) :`TraceChannel` "TraceTypeQuery1" :`DrawDebugType` "ForDuration"))
  (if _returnvalue_2
    (bind (_bblockinghit _binitialoverlap _time _distance _location _impactpoint _normal _impactnormal _physmat _hitactor) (`GameplayStatics.BreakHitResult` _outhit))
    (`GameplayStatics.ApplyPointDamage` _hitactor (`self.Damage`) _impactnormal _outhit _returnvalue self "/Script/Engine.DamageType")
    (`AISense_Damage.ReportDamageEvent` _hitactor _returnvalue (`self.Damage`) _location)))

(fn `UserConstructionScript`)