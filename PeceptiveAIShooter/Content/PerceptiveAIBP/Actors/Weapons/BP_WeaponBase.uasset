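; Base weapon actor that fires rounds on request, with gunshots and hits reported to AI perception.
; A DoOnce gate and FireRate timer throttle shots, calling RoundFired when the gate resets.
; Each shot spawns BulletClass at the arrow, plays sound and makes a "Gunshot" noise for Pawn owners.
; Damage comes from a debug-drawn hitscan along the mesh's forward vector, which also reports a damage event located at the trace start.
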(event `OnFireRequested`
  (bind _returnvalue (`SceneComponent.K2_GetComponentToWorld` (`self.Arrow`)))
  (`/Engine/EditorBlueprintResources/StandardMacros.DoOnce` false :!label _label
    (:`Completed`
      (`self.FireRound` _returnvalue (`KismetMathLibrary.TransformLocation` _returnvalue))
      (`KismetSystemLibrary.K2_SetTimer` null "FireReady" (`self.FireRate`)))))

(event `FireReady`
  (`self.RoundFired`)
  (goto _label :!via `Reset`))

(event `FireRound`
  (params (MuzzleTransform :type "Transform Structure (by ref)") (MuzzleLocation :type "Vector Structure (by ref)"))
  (bind _returnvalue (`self.GetInstigatorController` (`self.GetOwner`)))
  (bind _returnvalue_2 (`|SpawnActorFromClass` (`self.Bullet class`) MuzzleTransform "AdjustIfPossibleButAlwaysSpawn" "OverrideRootScale" null null))
  (`GameplayStatics.PlaySoundAtLocation` "/Game/FPSTemplate/FPWeapon/Audio/FirstPersonTemplateWeaponFire02.FirstPersonTemplateWeaponFire02" MuzzleLocation (struct) 0.1 1.0 0.0 null null null null)
  (bind _aspawn (cast `Pawn` (`self.GetOwner`))
    (:`then`
      (`self.MakeNoise` 1.0 _aspawn MuzzleLocation 0.0 "Gunshot"))
    (:`CastFailed`
      _))
  (bind _outhit (`KismetSystemLibrary.LineTraceSingle` MuzzleLocation (+ MuzzleLocation (* (`SceneComponent.GetForwardVector` (`self.SkeletalMesh`)) (`self.Range`))) "TraceTypeQuery2" false (`|MakeArray` _returnvalue_2 (`self.GetOwner`)) "ForDuration"))
  (bind (_bblockinghit _binitialoverlap _time _distance _location _impactpoint _normal _impactnormal _physmat _hitactor _hitcomponent _hitbonename _bonename _hititem _elementindex _faceindex _tracestart) (`GameplayStatics.BreakHitResult` _outhit))
  (if _bblockinghit
    (`GameplayStatics.ApplyDamage` _hitactor (`self.Damage`) _returnvalue self "/Script/Engine.DamageType")
    (`AISense_Damage.ReportDamageEvent` _hitactor _returnvalue (`self.Damage`) _tracestart)))

(fn `UserConstructionScript`)